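; Custom Game Instance that supplies player identity data from the online subsystem, apparently for a lobby.
; LoadPlayerInfofromSubsystem fills the LobbyPlayerInfo struct with the first local player's nickname and unique net ID as a string.
; GetPlayerAvatarImage converts an ID string to a Steam ID and returns the small friend avatar, falling back to a generic person texture when Steam is absent or the lookup fails.
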(event EventLoadPlayerInfofromSubsystem
  (bind _returnvalue (Game|GetPlayerController 0))
  (bind _uniquenetid (Class|AdvancedSessionsLibrary|GetUniqueNetID _returnvalue))
  (Utilities|Struct|SetmembersinLobbyPlayerInfo (Variables|Default|GetLobbyPlayerInfo) (Class|AdvancedIdentityLibrary|GetPlayerNickname _uniquenetid) (Class|AdvancedSessionsLibrary|UniqueNetIdtoString _uniquenetid)))

(fn GetPlayerAvatarImage
  (params (UniquePlayerIdString :type String))
  (if (Class|AdvancedSessionsLibrary|HasOnlineSubsystem "STEAM")
    (bind _returnvalue (Class|AdvancedSteamFriendsLibrary|GetSteamFriendAvatar (Class|AdvancedSteamFriendsLibrary|CreateSteamIDfromString UniquePlayerIdString) "SteamAvatar_Small")
      (:OnSuccess
        (return _returnvalue))
      (:OnFailure
        _)))
  (return "/Game/MenuSystem/Images/T_Person.T_Person"))